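; Tank pawn Blueprint that wires up the turret and barrel and lets the player orbit the aiming camera.
; On BeginPlay it passes the barrel and turret components to reference setters and assigns their static meshes.
; Azimuth input yaws a gimbal component while elevation input pitches the spring arm, both frame-rate independent via scaled delta time.
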(event `self.ReceiveBeginPlay`
  (`self.SetBarrelRefrence` (`self.TankBarrel`))
  (`self.SetTurretRefrence` (`self.TankTurret`))
  (`StaticMeshComponent.SetStaticMesh` (`self.TankTurret`) "/Game/Tank/BattleTanks_Content_Tank_tank_fbx_Turret.tank_fbx_Turret")
  (`StaticMeshComponent.SetStaticMesh` (`self.TankBarrel`) "/Game/Tank/BattleTanks_Content_Tank_tank_fbx_Barrel.tank_fbx_Barrel"))

(event `InputAxis|AimAzimuth`
  (params (AxisValue :type "Float (single-precision)"))
  ;[1 1 1] Camera Input Binding
  (`SceneComponent.K2_AddLocalRotation` (`self.Azimuth Gambal`) (`KismetMathLibrary.MakeRotator` 0.0 0.0 (* AxisValue (`GameplayStatics.GetWorldDeltaSeconds`) 100.0)) false false))

(event `InputAxis|AimElevation`
  (params (AxisValue :type "Float (single-precision)"))
  ;[1 1 1] Camera Input Binding
  (`SceneComponent.K2_AddLocalRotation` (`self.SpringArm`) (`KismetMathLibrary.MakeRotator` 0.0 (* AxisValue (`GameplayStatics.GetWorldDeltaSeconds`) 100.0)) false false))

(fn `UserConstructionScript`)